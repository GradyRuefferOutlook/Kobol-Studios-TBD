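; Player stats component that tracks current and max health and stamina through callable functions, with no active event logic.
; Decrease functions subtract without clamping; DecreaseHealth returns whether health has reached zero or below, while DecreaseStamina returns true on both branches.
; Increase functions cap the current value at its max.
; Raising max stamina also refills stamina, while raising max health leaves current health unchanged.
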(event EventBeginPlay)

(event EventTick
  (params (DeltaSeconds :type Float%20%28single-precision%29)))

(fn DecreaseHealth
  (params (Damage :type Float%20%28double-precision%29))
  (bind _output_get (Variables|Health|SetCurrentHealth (- (Variables|Health|GetCurrentHealth) Damage)))
  (if (<= _output_get 0.0)
    (return true)
    (else
      (return false))))

(fn IncreaseMaxHealth
  (params (Incremention :type Float%20%28double-precision%29))
  (Variables|Health|SetMaxHealth (+ (Variables|Health|GetMaxHealth) Incremention)))

(fn DecreaseStamina
  (params (Stamina%20Depleted :type Float%20%28double-precision%29))
  (Variables|Stamina|SetCurrentStamina (- (Variables|Stamina|GetCurrentStamina) Stamina%20Depleted))
  (if (<= (Variables|Stamina|GetCurrentStamina) 0.0)
    (return true)
    (else
      (return true))))

(fn IncreaseMaxStamina
  (params (Added%20Stamina :type Float%20%28double-precision%29))
  (bind _output_get (Variables|Stamina|SetMaxStamina (+ (Variables|Stamina|GetMaxStamina) Added%20Stamina)))
  (Variables|Stamina|SetCurrentStamina _output_get))

(fn IncreaseHealth
  (params (Healing :type Float%20%28double-precision%29))
  (bind _maxhealth (Variables|Health|GetMaxHealth))
  (bind _output_get (Variables|Health|SetCurrentHealth (+ (Variables|Health|GetCurrentHealth) Healing)))
  (if (>= _output_get _maxhealth)
    (Variables|Health|SetCurrentHealth _maxhealth)))

(fn IncreaseStamina
  (params (Rejuvination :type Float%20%28double-precision%29))
  (bind _maxstamina (Variables|Stamina|GetMaxStamina))
  (bind _output_get (Variables|Stamina|SetCurrentStamina (+ (Variables|Stamina|GetCurrentStamina) Rejuvination)))
  (if (>= _output_get _maxstamina)
    (Variables|Stamina|SetCurrentStamina _maxstamina)))